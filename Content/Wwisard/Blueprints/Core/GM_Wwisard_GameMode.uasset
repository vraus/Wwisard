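; Game mode for Wwisard that runs the chamfer door puzzle, win state and volume menu.
; Green chamfer events raise a counter and red ones lower it while below the required count; reaching it opens the level's A_Door once.
; Winning shows the win screen and unpossesses the player.
; BeginPlay binds events, creates widgets and resets Wwise RTPCs, adding a main widget inside that loop, once per RTPC.
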(event `self.ReceiveBeginPlay`
  (bind _returnvalue (`GameplayStatics.GetActorOfClass` "/Game/Wwisard/Blueprints/Actors/A_Door.A_Door_C"))
  (`/Engine/EditorBlueprintResources/StandardMacros.IsValid` _returnvalue
    (:`Is Valid`
      (set `self.Door` _returnvalue)
      (add `self.OnChamferGreen` (delegate `CheckGreenChamfer`))
      (add `self.OnChamferRed` (delegate `ComputeRedChamfer`))
      (bind _returnvalue_2 (`|CreateWidget` "/Game/Wwisard/UI/WB_WinScreen.WB_WinScreen_C"))
      (set `self.WinScreen` _returnvalue_2)
      (add `self.OnPlayerStepInWinArea` (delegate `Win`))
      (bind _returnvalue_3 (`|CreateWidget` "/Game/Wwisard/UI/WB_VolumeParam.WB_VolumeParam_C"))
      (bind _output_get (set `self.VolumeControlScreen` _returnvalue_3))
      (`UserWidget.AddToViewport` _output_get 0)
      (for _array_element (`self.RTPCs`)
        (`AkGameplayStatics.ResetRTPCValue` _array_element)
        (bind _returnvalue_4 (`|CreateWidget` "/Game/Wwisard/UI/WB_Main.WB_Main_C"))
        (`UserWidget.AddToViewport` _returnvalue_4 0)))
    (:`Is Not Valid`
      (`KismetSystemLibrary.PrintString` "A_Door class is not valid"))))

(event `ComputeRedChamfer`
  (if (< (`self.CurrentGreenChamfer`) (`self.MandatoryGreenChamfer`))
    (`/Engine/EditorBlueprintResources/StandardMacros.DecrementFloat` (`self.CurrentGreenChamfer`))))

(event `CheckGreenChamfer`
  (bind _result (`/Engine/EditorBlueprintResources/StandardMacros.IncrementFloat` (`self.CurrentGreenChamfer`))
    (:`  `
      (if (>= _result (`self.MandatoryGreenChamfer`))
        (`/Engine/EditorBlueprintResources/StandardMacros.DoOnce` false
          (:`Completed`
            (`/Game/Wwisard/Blueprints/Actors/A_Door.SetDoorOpened` (`self.Door`))))
        (else
          (`KismetSystemLibrary.PrintString` (`KismetStringLibrary.Conv_DoubleToString` _result)))))))

(event `Win`
  (`UserWidget.AddToViewport` (`self.WinScreen`) 0)
  (`Controller.UnPossess` (`GameplayStatics.GetPlayerController` 0)))

(event `ToggleDisplayVolumeMenu`
  (bind _volumecontrolscreen (`self.VolumeControlScreen`))
  (`Widget.SetVisibility` _volumecontrolscreen (select `ESlateVisibility` (`Widget.Visibility` _volumecontrolscreen) :`Visible` "Hidden" :`Collapsed` "Visible" :`Hidden` "Visible" :`HitTestInvisible` "Visible" :`SelfHitTestInvisible` "Visible" :!type "ESlateVisibility Enum")))

(fn `UserConstructionScript`)